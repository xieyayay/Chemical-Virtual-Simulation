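; Task manager actor for a step-by-step equipment operation training game with exam scoring, driven by DT_Tasks rows keyed on the current step.
; Equipment clicks are checked against single or ordered multi-step targets, showing images and playing the step's sequence on success.
; Wrong single-step clicks deduct score and log hints.
; It also updates HUD hints, advances after sequences, supports stepping back or auto-executing, and toggles ground guide actors.
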(event Custom|InitalGuide
  ;[0.15 0.15 0.15 0.5] 地上的指引
  (for _array_element (Variables|Default|GetZhiyin)
    (Rendering|SetActorHiddenInGame _array_element true))
  (Rendering|SetActorHiddenInGame (Utilities|Array|Get(acopy) (Variables|Default|GetZhiyin)) false) ; 第一个指引最开始显示
)

(event Custom|UpdateGuide
  (params (Zhiyin_Index :type Integer))
  (bind _zhiyin (Variables|Default|GetZhiyin))
  (bind _output (Utilities|Array|Get(acopy) _zhiyin Zhiyin_Index))
  ;[0.15 0.15 0.15 0.5] 地上的指引
  (if (!= Zhiyin_Index 0)
    (Rendering|SetActorHiddenInGame _output false) ; 显示
    (Variables|Default|SetUsedZhiYin _output)))

(event EventBeginPlay
  (bind _returnvalue (Actor|GetActorOfClass "/Game/ThirdPerson/Blueprints/BP_ThirdPersonGameMode.BP_ThirdPersonGameMode_C"))
  (Variables|Default|SetBP%20Third%20Person%20Mode _returnvalue)
  (CallFunction|InitalGuide))

(event EventTick
  (params (DeltaSeconds :type Float%20%28single-precision%29))
  (bind _returnvalue (Game|GetPlayerController 0))
  (bind _hudwidgetref (Variables|Default|GetHUDWidgetRef))
  (bind (_locationx _locationy) (Game|Player|GetMousePosition _returnvalue))
  (bind _txt_floatinghint (Variables|/Game/main_UI/RenWu_UI/WBP_TaskPanel2.WBP_TaskPanel2_C|GetTxt_FloatingHint _hudwidgetref))
  (if (Utilities|Enum|Equal(Enum) (Widget|GetVisibility _txt_floatinghint) "Visible")
    (Class|Widget|SetRenderTranslation _txt_floatinghint (Math|Vector2D|MakeVector2D (+ _locationx 2e+01) (+ _locationy 2e+01)))))

(fn ConstructionScript)

(fn HandleEquipmentInteract
  (params (Equipment :type BP%20Interact%20Object%20Reference) (PartID :type Integer))
  (bind _currenttaskstep (Variables|Default|GetCurrentTaskStep))
  (bind _currenttaskstep_2 (Variables|Default|GetCurrentTaskStep))
  (bind _bp_third_person_mode (Variables|Default|GetBP%20Third%20Person%20Mode))
  (bind _multistepprogressmap (Variables|Default|GetMultiStepProgressMap))
  (bind _equipmentid (Variables|/Game/UI/BP/interact/BP_l/BP_interact.BP_interact_C|GetEquipmentID Equipment))
  (bind _multistepprogressmap_2 (Variables|Default|GetMultiStepProgressMap))
  (bind _value (Utilities|Map|Find _multistepprogressmap _currenttaskstep_2))
  (bind _hudwidget (Variables|/Game/ThirdPerson/Blueprints/BP_ThirdPersonGameMode.BP_ThirdPersonGameMode_C|GetHUDWidget _bp_third_person_mode))
  (Variables|Default|SetPart%20ID PartID)
  (bind _returnvalue (Utilities|GetDataTableRow "/Game/main_UI/RenWu_UI/BP_rw/DT_Tasks.DT_Tasks" (Utilities|String|StringToName (Utilities|String|ToString(Integer) (Variables|Default|GetCurrentTaskStep))))
    (:then
      (Utilities|IsValid Equipment
        (:Is%20Valid
          (Default|Tips (Variables|/Game/ThirdPerson/Blueprints/BP_ThirdPersonGameMode.BP_ThirdPersonGameMode_C|GetHUDWidget (Variables|Default|GetBP%20Third%20Person%20Mode)) _equipmentid)
          (Variables|Default|SetCurrent%20Click%20Index _value)
          (bind _output_get (Variables|Default|SetIs%20Completed (.bIsCompleted (Utilities|Struct|BreakS_TaskStep _returnvalue))))
          (if _output_get ; 0
            (return)
            (else
              (bind _output_get_2 (Variables|Default|SetIs%20Multi%20Step (.bIsMultiStep (Utilities|Struct|BreakS_TaskStep _returnvalue))))
              (if _output_get_2 ; 多步判断
                (if (< _value (Utilities|Array|Length (.TargetEquipmentIDs (Utilities|Struct|BreakS_TaskStep _returnvalue)))) ; 多步条件判断1
                  (bind _output_get_3 (Variables|Default|SetOnclick_milt_pipei (== _equipmentid (Utilities|Array|Get(acopy) (.TargetEquipmentIDs (Utilities|Struct|BreakS_TaskStep _returnvalue)) _value))))
                  (if _output_get_3 ; 多步条件判断2
                    ;[1 1 1] 新增映射
                    (Utilities|Map|Add _multistepprogressmap_2 _currenttaskstep (+ (.Value (Utilities|Map|Find _multistepprogressmap_2 _currenttaskstep)) 1))
                    (Default|ShowTaskImage _hudwidget (.Value (Utilities|Map|Find (.duobu_image (Utilities|Struct|BreakS_TaskStep _returnvalue)) _value))) ; 多步图片播放
                    ;[1 1 1] 点击指定一起后最终播放（依次点击后播放一次
                    (if (>= _value (Utilities|Array|Length (.TargetEquipmentIDs (Utilities|Struct|BreakS_TaskStep _returnvalue)))) ; 多部条件判断3(finish
                      (CallFunction|CompleteCurrentStep :!pinned true) ; 多步完结
                      (else
                        (CallFunction|UpdateTaskHint))))
                  (else
                    (return)))
                (elif (and (Utilities|Enum|Equal(Enum) (Utilities|String|ToString(Integer) _equipmentid) (Utilities|String|ToString(Integer) (.TargetEquipmentID (Utilities|Struct|BreakS_TaskStep _returnvalue)))) (or (== (.TargetPartID (Utilities|Struct|BreakS_TaskStep _returnvalue)) 0) (== PartID (.TargetPartID (Utilities|Struct|BreakS_TaskStep _returnvalue))))) ; 单步逻辑判断（finish
                  (Default|ShowTaskImage _hudwidget (.image (Utilities|Struct|BreakS_TaskStep _returnvalue))) ; 单步图片播放
                  (CallFunction|CompleteCurrentStep :!pinned true) ; 单步判断完成
                  (else
                    ;[1 1 1] 考试模式
                    (bind _foundwidgets (Widget|GetAllWidgetsOfClass "/Game/Game_MoShi/WBP_score.WBP_score_C" true))
                    (bind _当前总分 (Default|UpdateScoreDisplay _foundwidgets 1))
                    (bind _扣分 (Default|CurrentKoufen _foundwidgets 1))
                    (bind _now_tishi (Default|GiveTishi _foundwidgets (Utilities|String|ToString(Text) (.jian_TaskDescription (Utilities|Struct|BreakS_TaskStep _returnvalue)))))
                    (Utilities|Array|Add (Variables|Default|GetSum_提示) _now_tishi)
                    (Utilities|Array|Add (Variables|Default|GetSum_扣分) _扣分)
                    (Default|CallAddList)
                    (if (<= _当前总分 0)
                      (Default|创建0分失败控件 _foundwidgets))))))))))))

(fn CompleteCurrentStep
  (bind _returnvalue (Utilities|GetDataTableRow "/Game/main_UI/RenWu_UI/BP_rw/DT_Tasks.DT_Tasks" (Utilities|String|StringToName (Utilities|String|ToString(Integer) (Variables|Default|GetCurrentTaskStep))))
    (:then
      (Variables|Default|SetIs%20Completed true)
      (Utilities|IsValid (.TargetSequence (Utilities|Struct|BreakS_TaskStep _returnvalue))
        (:Is%20Valid
          (Default|PlayLevelSequence (Variables|Default|GetSequenceManagerRef) (.TargetSequence (Utilities|Struct|BreakS_TaskStep _returnvalue)) (.TargetEquipmentID (Utilities|Struct|BreakS_TaskStep _returnvalue)) (.UI_Widget (Utilities|Struct|BreakS_TaskStep _returnvalue)) 0 (.sound (Utilities|Struct|BreakS_TaskStep _returnvalue)) (.zhi_yin (Utilities|Struct|BreakS_TaskStep _returnvalue)) (.zhi_yin_Index (Utilities|Struct|BreakS_TaskStep _returnvalue))))))))

(fn UpdateTaskHint
  (bind _hudwidgetref (Variables|Default|GetHUDWidgetRef))
  (bind _returnvalue (Utilities|GetDataTableRow "/Game/main_UI/RenWu_UI/BP_rw/DT_Tasks.DT_Tasks" (Utilities|String|StringToName (Utilities|String|ToString(Integer) (Variables|Default|GetCurrentTaskStep))))
    (:then
      (Utilities|IsValid (Variables|Default|GetHUDWidgetRef)
        (:Is%20Valid
          (if (not (.bIsCompleted (Utilities|Struct|BreakS_TaskStep _returnvalue)))
            (if (.bIsMultiStep (Utilities|Struct|BreakS_TaskStep _returnvalue))
              (for _array_element (Variables|Default|GetEquipmentRefs)
                (if (== (Variables|/Game/UI/BP/interact/BP_l/BP_interact.BP_interact_C|GetEquipmentID _array_element) (Utilities|Array|Get(acopy) (.TargetEquipmentIDs (Utilities|Struct|BreakS_TaskStep _returnvalue)) (.Value (Utilities|Map|Find (Variables|Default|GetMultiStepProgressMap) (Variables|Default|GetCurrentTaskStep)))))
                  (bind _name (Default|GetEquipmentName _array_element))
                  (bind _output_get (Variables|Default|SetEquipt_Name _name))
                  (Default|SetTaskHintText _hudwidgetref (Utilities|Text|FormatText "此步骤需依次点击仪器 
请点击{仪器名称}" _output_get) (.Title (Utilities|Struct|BreakS_TaskStep _returnvalue)) (.juti_TaskDescription (Utilities|Struct|BreakS_TaskStep _returnvalue)) (.TaskCompleted (Utilities|Struct|BreakS_TaskStep _returnvalue)) (.OnTaskCompleted？ (Utilities|Struct|BreakS_TaskStep _returnvalue)))
                  (Development|PrintString "多部更新UI")))
              (else
                (Default|SetTaskHintText _hudwidgetref (.jian_TaskDescription (Utilities|Struct|BreakS_TaskStep _returnvalue)) (.Title (Utilities|Struct|BreakS_TaskStep _returnvalue)) (.juti_TaskDescription (Utilities|Struct|BreakS_TaskStep _returnvalue)) (.TaskCompleted (Utilities|Struct|BreakS_TaskStep _returnvalue)) (.OnTaskCompleted？ (Utilities|Struct|BreakS_TaskStep _returnvalue)))))))
        (:Is%20Not%20Valid
          (return))))))

(fn ExecuteCurrentStepOperation
  (bind _returnvalue (Utilities|GetDataTableRow "/Game/main_UI/RenWu_UI/BP_rw/DT_Tasks.DT_Tasks" (Utilities|String|StringToName (Utilities|String|ToString(Integer) (Variables|Default|GetCurrentTaskStep))))
    (:then
      (if (and (not (.bIsCompleted (Utilities|Struct|BreakS_TaskStep _returnvalue))) (Utilities|IsValid (.TargetSequence (Utilities|Struct|BreakS_TaskStep _returnvalue))))
        (Default|ShowTaskImage (Variables|/Game/ThirdPerson/Blueprints/BP_ThirdPersonGameMode.BP_ThirdPersonGameMode_C|GetHUDWidget (Variables|Default|GetBP%20Third%20Person%20Mode)) (.image (Utilities|Struct|BreakS_TaskStep _returnvalue))) ; 单步图片播放
        (Default|Tips (Variables|/Game/ThirdPerson/Blueprints/BP_ThirdPersonGameMode.BP_ThirdPersonGameMode_C|GetHUDWidget (Variables|Default|GetBP%20Third%20Person%20Mode)) (.TargetEquipmentID (Utilities|Struct|BreakS_TaskStep _returnvalue)))
        (Default|PlayLevelSequence (Variables|Default|GetSequenceManagerRef) (.TargetSequence (Utilities|Struct|BreakS_TaskStep _returnvalue)) (.TargetEquipmentID (Utilities|Struct|BreakS_TaskStep _returnvalue)) (.UI_Widget (Utilities|Struct|BreakS_TaskStep _returnvalue)) (.image (Utilities|Struct|BreakS_TaskStep _returnvalue)) (.sound (Utilities|Struct|BreakS_TaskStep _returnvalue)) (.zhi_yin (Utilities|Struct|BreakS_TaskStep _returnvalue)))))))

(fn GotoPreviousStep
  (bind _currenttaskstep (Variables|Default|GetCurrentTaskStep))
  (bind _returnvalue (Utilities|GetDataTableRow "/Game/main_UI/RenWu_UI/BP_rw/DT_Tasks.DT_Tasks" (Utilities|String|StringToName (Utilities|String|ToString(Integer) (Variables|Default|GetCurrentTaskStep))))
    (:then
      (if (> (Variables|Default|GetCurrentTaskStep) 1)
        (Math|Integer|DecrementInt _currenttaskstep
          (:%20%20
            (Variables|Default|SetIs%20Completed false)
            (Utilities|Map|Add (Variables|Default|GetMultiStepProgressMap) _currenttaskstep 0)
            (CallFunction|UpdateTaskHint)
            (Default|ShowTaskImage (Variables|/Game/ThirdPerson/Blueprints/BP_ThirdPersonGameMode.BP_ThirdPersonGameMode_C|GetHUDWidget (Variables|Default|GetBP%20Third%20Person%20Mode)) (.image (Utilities|Struct|BreakS_TaskStep _returnvalue))) ; 多步图片播放
          ))))))

(fn OnSequenceCompleted
  (Variables|Default|SetCurrentTaskStep (+ (Variables|Default|GetCurrentTaskStep) 1))
  (bind _returnvalue (Utilities|GetDataTableRow "/Game/main_UI/RenWu_UI/BP_rw/DT_Tasks.DT_Tasks" (Utilities|String|StringToName (Utilities|String|ToString(Integer) (Variables|Default|GetCurrentTaskStep))))
    (:then
      (if (<= (Variables|Default|GetCurrentTaskStep) (.StepNumber (Utilities|Struct|BreakS_TaskStep _returnvalue)))
        (CallFunction|UpdateTaskHint)))))

(fn ShowOperationHint
  (params (Equipment :type BP%20Interact%20Object%20Reference)))

(fn HideOperationHint
  (Default|HideFloatingHint (Variables|Default|GetHUDWidgetRef)))