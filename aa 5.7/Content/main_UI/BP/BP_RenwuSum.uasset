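; BP_RenwuSum is an input-driven Blueprint that toggles two full-screen-layer UI widgets: a task book and an experiment report.
; Tab toggles the book widget, fed by Book_DataTable, and the ShowManual action (noted as L) toggles WBP_shiyanbaogao.
; Each toggle creates or removes its widget, using the stored reference as open state.
; A helper fetches BP_playercontroller to switch input mode and cursor visibility accordingly.
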(event Input|ActionEvents|InputActionShowManual
  (params (Key :type Key%20Structure :default "None"))
  (bind _asbp_playercontroller (CallFunction|新函数))
  ;[1 1 1] 按L打开实验报告
  (:Pressed
    (bind _shiyanbaogao (Variables|Default|Getshiyanbaogao)
      (:then
        (Widget|RemovefromParent _shiyanbaogao)
        (Variables|Default|Setshiyanbaogao 0)
        (Default|SetInputMode _asbp_playercontroller "NewEnumerator0" false))
      (:else
        (bind _returnvalue (UserInterface|CreateWidget "/Game/main_UI/over_shiyanbaogao/WBP_shiyanbaogao.WBP_shiyanbaogao_C" (Game|GetPlayerController 0)))
        (UserInterface|Viewport|AddtoViewport _returnvalue 100)
        (Variables|Default|Setshiyanbaogao _returnvalue)
        (Default|SetInputMode _asbp_playercontroller "NewEnumerator1" true)))))

(event Input|KeyboardEvents|Tab
  (params (Key :type Key%20Structure :default "None"))
  (bind _asbp_playercontroller (CallFunction|新函数))
  ;[1 1 1] Tab 键 添加和移除视口
  (:Pressed
    (bind _renwushu1 (Variables|Default|GetRenWuShu1)
      (:then
        (Widget|RemovefromParent _renwushu1)
        (Variables|Default|SetRenWuShu1 0)
        (Default|SetInputMode _asbp_playercontroller "NewEnumerator0" false))
      (:else
        (bind _returnvalue (UserInterface|CreateWidget "/Game/main_UI/RenWuShu/renwushu1.renwushu1_C" (Game|GetPlayerController 0) 0 "/Game/main_UI/RenWuShu/Book_DataTable.Book_DataTable"))
        (UserInterface|Viewport|AddtoViewport _returnvalue 100)
        (Variables|Default|SetRenWuShu1 _returnvalue)
        (Default|SetInputMode _asbp_playercontroller "NewEnumerator1" true)))))

(fn 新函数
  (return (.AsBP%20Playercontroller (Utilities|Casting|CastToBP_playercontroller (Game|GetPlayerController 0)))))